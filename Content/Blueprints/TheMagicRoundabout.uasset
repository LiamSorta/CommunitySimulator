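; TheMagicRoundabout is a rotating lift that carries out a one-way upward journey when E is pressed.
; At start it sets a target 1650 units up and disables wall collision; E re-enables it.
; Tick then raises and spins it by fixed per-frame steps, so speed depends on frame rate.
; At the top it stops, reveals a set of hidden actors, and hides the door and disables its collision.
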(event `self.ReceiveBeginPlay`
  (`self.EnableInput` (`GameplayStatics.GetPlayerController` 0))
  (set `self.TargetHeight` (+ (`self.K2_GetActorLocation`) (0.0 0.0 1650.0)))
  (`self.DisableWalls`))

(event `Key|E`
  (params (Key :type "Key Structure" :default "AnyKey"))
  (:`Pressed`
    (set `self.StartEvent` true)
    (`self.EnableWalls`)))

(event `self.ReceiveTick`
  (params (DeltaSeconds :type "Float (single-precision)"))
  (if (`self.StartEvent`)
    (if (not (`self.IsDone`))
      (`self.JourneyProgress`))))

(fn `DisableWalls`
  (for _array_element (`self.AllWalls`)
    (`self.SetActorEnableCollision` _array_element false)))

(fn `EnableWalls`
  (for _array_element (`self.AllWalls`)
    (`self.SetActorEnableCollision` _array_element true)))

(fn `JourneyComplete`
  (bind _door (`self.Door`))
  (set `self.IsDone` true)
  (for _array_element (`self.ThingsToShow`)
    (`self.SetActorHiddenInGame` _array_element false))
  (`self.SetActorHiddenInGame` _door true)
  (`self.SetActorEnableCollision` _door false))

(fn `JourneyProgress`
  (bind _returnvalue (`self.K2_GetActorLocation`))
  (if (> (.z (`self.TargetHeight`)) (.z _returnvalue))
    (`self.K2_SetActorLocation` (+ _returnvalue (0.0 0.0 1.3)))
    (`self.K2_AddActorLocalRotation` (`self.Mesh`) (struct :`Yaw` 1.3) false false)
    (else
      (`self.JourneyComplete`))))

(fn `UserConstructionScript`)